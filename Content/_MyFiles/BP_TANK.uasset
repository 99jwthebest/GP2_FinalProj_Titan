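; BP_TANK is a tank AI pawn that wanders the level, apparently a work in progress.
; Tick runs through a five-second Delay, then, while CanSeePlayer is false, moves it to a random reachable nearby point and prints debug text.
; PawnSensing is present, but OnSeePawn is empty and the player-chase logic is disconnected, so CanSeePlayer is never set true.
; Rotation smoothing and timeline experiments are also left unwired.
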(event `self.PawnSensing.OnSeePawn`
  (params (Pawn :type "Pawn Object Reference")))

(event `self.ReceiveTick`
  (params (DeltaSeconds :type "Float (single-precision)"))
  (`KismetSystemLibrary.Delay` 5.0)
  (`KismetSystemLibrary.PrintString` "Hello")
  (if (not (`self.CanSeePlayer`))
    (bind _output_get (set `self.OldRotation` (`self.GetControlRotation`)))
    (`KismetSystemLibrary.PrintString` (`KismetStringLibrary.Conv_RotatorToString` _output_get))
    (`|AIMoveTo` self (`NavigationSystemV1.K2_GetRandomReachablePointInRadius` (`self.K2_GetActorLocation`) 2000.0 null null) null)))

(fn `UserConstructionScript`)