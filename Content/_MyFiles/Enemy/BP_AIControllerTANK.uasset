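; AI controller for the TANK enemy that runs its behavior tree and feeds perception results into the blackboard.
; On BeginPlay it starts BP_BehaviorTreeTANK and seeds LastKnownLoc with the controlled pawn's location.
; Perception updates set bSeenPlayer from whether the stimulus was sensed, clearing bLostPlayer on success and storing the stimulus location as LastKnownLoc on loss.
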(event `self.ReceiveBeginPlay`
  (`self.RunBehaviorTree` "/Game/_MyFiles/Enemy/BP_BehaviorTreeTANK.BP_BehaviorTreeTANK")
  (`BlackboardComponent.SetValueAsVector` (`AIBlueprintHelperLibrary.GetBlackboard` null) "LastKnownLoc" (`self.K2_GetActorLocation` (`self.K2_GetPawn`))))

(event `self.AIPerception.OnTargetPerceptionUpdated`
  (params (Actor :type "Actor Object Reference") (Stimulus :type "AIStimulus Structure"))
  (bind (_age _expirationage _strength _stimuluslocation _receiverlocation _tag _bsuccessfullysensed) (break `AIStimulus` Stimulus))
  (bind _returnvalue (`AIBlueprintHelperLibrary.GetBlackboard` null))
  (`BlackboardComponent.SetValueAsBool` (`AIBlueprintHelperLibrary.GetBlackboard` null) "bSeenPlayer" _bsuccessfullysensed)
  (if _bsuccessfullysensed
    (`BlackboardComponent.SetValueAsBool` _returnvalue "bLostPlayer" false)
    (else
      (`BlackboardComponent.SetValueAsVector` _returnvalue "LastKnownLoc" _stimuluslocation))))

(fn `UserConstructionScript`)