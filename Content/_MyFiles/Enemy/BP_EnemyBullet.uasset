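; BP_EnemyBullet is an enemy projectile that launches itself at the player with lead targeting.
; On BeginPlay it predicts the player's position from their velocity and a travel time of distance over ProjectileSpeed.
; It feeds that point into SuggestProjectileVelocity, with debug drawing enabled, to set the ProjectileMovement velocity and rotates to follow it.
; The bullet destroys itself after a short delay and contains no hit or damage logic.
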(event `self.ReceiveBeginPlay`
  (bind _returnvalue (`GameplayStatics.GetPlayerCharacter` 0))
  (bind _projectilemovement (`self.ProjectileMovement`))
  (bind _projectilespeed (`self.ProjectileSpeed`))
  (bind _tossvelocity (`GameplayStatics.BlueprintSuggestProjectileVelocity` (`self.K2_GetActorLocation`) (+ (`self.K2_GetActorLocation` _returnvalue) (* (`self.GetVelocity` _returnvalue) (/ (`self.GetDistanceTo` _returnvalue) _projectilespeed))) _projectilespeed 0.0 "DoNotTrace" 0.0 false true))
  (set `MovementComponent.Velocity` _tossvelocity _projectilemovement)
  (set `ProjectileMovementComponent.bRotationFollowsVelocity` true _projectilemovement)
  (`KismetSystemLibrary.Delay` 2.5)
  (`self.K2_DestroyActor`))

(fn `UserConstructionScript`)