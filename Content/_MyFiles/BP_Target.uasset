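; BP_Target is a shootable target that registers itself with the first-person character by incrementing its Target count on BeginPlay.
; When hit by an actor tagged "projectile", it calls HitTarget on that character and destroys itself.
; If CanMove is set, the construction script configures InterpToMovement with two relative control points and a duration so the target moves between them.
; An emitter spawn node is left unconnected.
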(event `self.ReceiveBeginPlay`
  (bind _asbp_first_person_character (cast `/Game/FirstPerson/Blueprints/BP_FirstPersonCharacter` (`GameplayStatics.GetPlayerCharacter` 0)))
  (bind _output_get (set `self.As BP First Person Character` _asbp_first_person_character))
  (bind _result (`/Engine/EditorBlueprintResources/StandardMacros.IncrementInt` (`GP2_JH_PersonalProjCharacter.Target` _output_get))
    (:`  `
      (set `GP2_JH_PersonalProjCharacter.Target` _result _output_get))))

(event `self.ReceiveHit`
  (params (MyComp :type "PrimitiveComponent Object Reference") (Other :type "Actor Object Reference") (OtherComp :type "PrimitiveComponent Object Reference") (bSelfMoved :type Boolean) (HitLocation :type "Vector Structure") (HitNormal :type "Vector Structure") (NormalImpulse :type "Vector Structure") (Hit :type "HitResult Structure (by ref)"))
  (if (`self.ActorHasTag` Other "projectile")
    (`/Game/FirstPerson/Blueprints/BP_FirstPersonCharacter.HitTarget` (`self.As BP First Person Character`))
    (`self.K2_DestroyActor`)))

(fn `UserConstructionScript`
  (bind _interptomovement (`self.InterpToMovement`))
  (if (`self.CanMove`)
    (set `InterpToMovementComponent.ControlPoints` (`|MakeArray` (make `InterpControlPoint` (`self.Location1`)) (make `InterpControlPoint` (`self.Location2`))) _interptomovement)
    (set `InterpToMovementComponent.Duration` (`self.Duration`) _interptomovement)))